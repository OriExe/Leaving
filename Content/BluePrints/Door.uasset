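; Interactable door Blueprint that swings open and shut, with an on-screen "Press E" prompt that matches its state.
; InteractionFunction hides the prompt, then branches on IsOpen to play the DoorOpening timeline with a sound or reverse it silently, lerping the door mesh's yaw.
; When the timeline finishes it flips IsOpen; after opening, a short delay loops back to auto-close the door.
; Actor overlap events show and hide the prompt.
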(event Collision|EventActorBeginOverlap
  (params (OtherActor :type Actor%20Object%20Reference))
  ;[1 1 1] Show and Hide Interact Text
  (if (Variables|Default|GetisOpen)
    (CallFunction|ShowInteractText "Press E to close Door")
    (else
      (CallFunction|ShowInteractText "Press E to open Door"))))

(event EventInteractionFunction
  ;[1 1 1] Open and close Door
  (CallFunction|HideInteractText)
  (if (Variables|Default|GetisOpen) :!label _label
    (bind _door (Timeline|Door%20Opening Reverse)
      (:Update
        (Transformation|SetRelativeRotation (Variables|Default|GetSM_Door) (Math|Rotator|MakeRotator 0.0 0.0 (Math|Float|Lerp 0.0 9e+01 _door)) false false))
      (:Finished
        (if (Variables|Default|GetisOpen)
          (Variables|Default|SetisOpen false)
          (else
            (Variables|Default|SetisOpen true)
            ;[1 1 1] Auto Close door
            (Utilities|FlowControl|Delay 2.5) ; Automatically closes door
            (if (Variables|Default|GetisOpen)
              (goto _label))))))
    (else
      (Audio|Components|Audio|Play (Variables|Default|GetDoor_open) 0.0)
      (Timeline|Door%20Opening Play))))

(event Collision|EventActorEndOverlap
  (params (OtherActor :type Actor%20Object%20Reference))
  ;[1 1 1] Show and Hide Interact Text
  (CallFunction|HideInteractText))

(fn ConstructionScript)