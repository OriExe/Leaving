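; isPlayerInside is an overlap-driven actor that changes the rain sound, apparently for when the player is inside or outside.
; On BeginPlay it creates a persistent 2D rain audio component and starts it.
; Overlap begin lowers its Pitch float parameter and overlap end restores it, each restarting playback from the beginning.
; The overlap events do not check which actor triggered them.
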(event EventBeginPlay
  (bind _returnvalue (Audio|CreateSound2D "/Game/Sounds/RainSound.RainSound" 1.0 1.0 0.0 0 false false))
  (bind _output_get (Variables|Default|SetRainSound _returnvalue))
  (Audio|Components|Audio|Play _output_get 0.0))

(event Collision|EventActorEndOverlap
  (params (OtherActor :type Actor%20Object%20Reference))
  (Audio|Parameter|SetFloatParameter (Variables|Default|GetRainSound) "Pitch" 1.0 :!class /Script/Engine.AudioComponent)
  (Audio|Components|Audio|Play (Variables|Default|GetRainSound) 0.0))

(event Collision|EventActorBeginOverlap
  (params (OtherActor :type Actor%20Object%20Reference))
  (Audio|Parameter|SetFloatParameter (Variables|Default|GetRainSound) "Pitch" 0.4 :!class /Script/Engine.AudioComponent)
  (Audio|Components|Audio|Play (Variables|Default|GetRainSound) 0.0))

(fn ConstructionScript)