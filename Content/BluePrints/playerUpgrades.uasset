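; Player upgrade functions that trade movement speed against money gain on the GamePlayer, found through GetActorOfClass.
; IncreaseSpeedMultiplier scales the current MaxWalkSpeed, so repeated calls compound, and resets MoneyMultiplier to 1.
; IncreaseMoneyMultiplier adds its parameter to MoneyMultiplier and restores MaxWalkSpeed to DefaultWalkSpeed.
; Each upgrade therefore cancels the other, leaving only one bonus active at a time.
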(fn IncreaseSpeedMultiplier
  (params (A :type Integer))
  ;[0.3664 0.7106 1] Increase Speed Gained
  (bind _returnvalue (Actor|GetActorOfClass 0 "/Game/BluePrints/GamePlayer.GamePlayer_C"))
  (Variables|/Script/Engine.CharacterMovementComponent|SetMaxWalkSpeed (Variables|/Script/Engine.Character|GetCharacterMovement _returnvalue) (* A (Variables|/Script/Engine.CharacterMovementComponent|GetMaxWalkSpeed (Variables|/Script/Engine.Character|GetCharacterMovement _returnvalue))))
  ;;[1 1 1] LowerMoneyMultiplier
  (bind _returnvalue_2 (Actor|GetActorOfClass 0 "/Game/BluePrints/GamePlayer.GamePlayer_C"))
  (Variables|/Game/BluePrints/GamePlayer.GamePlayer_C|SetmoneyMultiplier _returnvalue_2 1))

(fn IncreaseMoneyMultiplier
  (params (B :type Integer))
  ;[0.01255 0.5156 0] Increase Money gained
  (bind _returnvalue (Actor|GetActorOfClass 0 "/Game/BluePrints/GamePlayer.GamePlayer_C"))
  (Variables|/Game/BluePrints/GamePlayer.GamePlayer_C|SetmoneyMultiplier _returnvalue (+ (Variables|/Game/BluePrints/GamePlayer.GamePlayer_C|GetmoneyMultiplier _returnvalue) B))
  ;;[1 1 1] Lower Speed Multiplier
  (Variables|/Script/Engine.CharacterMovementComponent|SetMaxWalkSpeed (Variables|/Script/Engine.Character|GetCharacterMovement _returnvalue) (Variables|/Game/BluePrints/GamePlayer.GamePlayer_C|GetdefaultWalkSpeed _returnvalue)))