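; MoneyMultiplierBoost is a one-use pickup that sells a money gain boost for €10.
; Overlap shows or hides the interact prompt, and InteractionFunction finds the GamePlayer to run the Can Player Afford_2 check.
; That check calls SetScore with -10 when Score covers the cost, otherwise showing a refusal message.
; A successful purchase calls IncreaseMoneyMultiplier with 1 and destroys the actor.
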(event EventBeginPlay)

(event Collision|EventActorBeginOverlap
  (params (OtherActor :type Actor%20Object%20Reference))
  (CallFunction|ShowInteractText "Press E to spend €10 to double your money gain"))

(event EventTick
  (params (DeltaSeconds :type Float%20%28single-precision%29)))

(event Collision|EventActorEndOverlap
  (params (OtherActor :type Actor%20Object%20Reference))
  (CallFunction|HideInteractText))

(event EventInteractionFunction
  (bind _returnvalue (Actor|GetActorOfClass "/Game/BluePrints/GamePlayer.GamePlayer_C"))
  (|CanPlayerAfford_2 _returnvalue
    (:true
      (CallFunction|IncreaseMoneyMultiplier 1)
      (Actor|DestroyActor))))

(fn ConstructionScript)