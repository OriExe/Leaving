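; Stealable valuable item actor that adds to the player's stash and extends the countdown when taken.
; Actor overlap shows or hides a steal prompt.
; Its interaction event passes the item's Value to GamePlayer's sell value, calls a helper that increases the HUD countdown timer, then destroys the item.
; The helper reaches the timer by casting player 0's HUD to HudDefault and going through its PlayerHud.
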(event EventBeginPlay)

(event Collision|EventActorBeginOverlap
  (params (OtherActor :type Actor%20Object%20Reference))
  ;[1 1 1] Interact
  (CallFunction|ShowInteractText "Press E to Steal Item"))

(event Collision|EventActorEndOverlap
  (params (OtherActor :type Actor%20Object%20Reference))
  ;[1 1 1] Interact
  (CallFunction|HideInteractText))

(event EventInteractionFunction
  ;[1 1 1] Add Value to player's stash
  (bind _returnvalue (Actor|GetActorOfClass "/Game/BluePrints/GamePlayer.GamePlayer_C"))
  (Default|UpdateSellValue _returnvalue (Variables|Default|GetValue))
  (|IncreaseTimerby5_2)
  (Actor|DestroyActor))

(fn ConstructionScript)