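; Pawn shop interactable where the player sells carried items for score, showing prompts on overlap.
; On interaction, it passes the GamePlayer's SellValue to SetScore, negates it through UpdateSellValue, or reports nothing to sell.
; A successful sale also destroys its Cube and every CLight actor in the level, then adds time to the HUD countdown timer.
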(event Collision|EventActorBeginOverlap
  (params (OtherActor :type Actor%20Object%20Reference))
  ;[1 1 1] Interact
  (CallFunction|ShowInteractText "Press E to sell your items"))

(event EventInteractionFunction
  ;[1 1 1] Pawn Shop Sell
  (bind _returnvalue (Actor|GetActorOfClass "/Game/BluePrints/GamePlayer.GamePlayer_C"))
  (bind _output_get (Variables|Default|SetPlayerREF _returnvalue))
  (if (> (Variables|/Game/BluePrints/GamePlayer.GamePlayer_C|GetsellValue _output_get) 0)
    (Default|SetScore (Variables|Default|GetPlayerREF) (Variables|/Game/BluePrints/GamePlayer.GamePlayer_C|GetsellValue (Variables|Default|GetPlayerREF)))
    (Default|UpdateSellValue (Variables|Default|GetPlayerREF) (* (Variables|/Game/BluePrints/GamePlayer.GamePlayer_C|GetsellValue (Variables|Default|GetPlayerREF)) -1))
    (CallFunction|ShowInteractText "SOLD!!")
    (|Destroyall)
    ;;[1 1 1] Increase time
    (bind _ashud_default (Utilities|Casting|CastToHudDefault (HUD|GetHUD (Game|GetPlayerController 0))))
    (Variables|/Game/UserInteraface/Countdown_Timer.Countdown_Timer_C|SetCountdown (Variables|/Game/UserInteraface/PlayerHeadsUpDisplay.PlayerHeadsUpDisplay_C|GetCountdown_Timer (Variables|/Game/UserInteraface/HudDefault.HudDefault_C|GetPlayerHud _ashud_default)) (+ 5.0 (Variables|/Game/UserInteraface/Countdown_Timer.Countdown_Timer_C|GetCountdown (Variables|/Game/UserInteraface/PlayerHeadsUpDisplay.PlayerHeadsUpDisplay_C|GetCountdown_Timer (Variables|/Game/UserInteraface/HudDefault.HudDefault_C|GetPlayerHud _ashud_default)))))
    (else
      (CallFunction|ShowInteractText "You have nothing to sell"))))

(event Collision|EventActorEndOverlap
  (params (OtherActor :type Actor%20Object%20Reference))
  ;[1 1 1] Interact
  (CallFunction|HideInteractText))

(fn ConstructionScript)