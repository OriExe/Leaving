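; interactTextAppear is a helper Blueprint that shows and hides interaction text on the player's HUD.
; ShowInteractText and HideInteractText each cast the HUD of player controller 0 to HudDefault and forward the call to its PlayerHud, passing the string through when showing.
; Both do nothing if that cast fails, and only the first player's HUD is ever targeted.
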(fn ShowInteractText
  (params (InString :type String))
  (bind _ashud_default (Utilities|Casting|CastToHudDefault (HUD|GetHUD (Game|GetPlayerController 0))))
  (Default|ShowInteractText (Variables|/Game/UserInteraface/HudDefault.HudDefault_C|GetPlayerHud _ashud_default) InString))

(fn HideInteractText
  (bind _ashud_default (Utilities|Casting|CastToHudDefault (HUD|GetHUD (Game|GetPlayerController 0))))
  (Default|HideInteractText (Variables|/Game/UserInteraface/HudDefault.HudDefault_C|GetPlayerHud _ashud_default)))