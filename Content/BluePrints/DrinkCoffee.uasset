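; Interactable actor that lets the player drink the coffee they are carrying to gain a coffee boost.
; On interaction it finds the GamePlayer and, if its Coffee component is visible, hides it, sets CoffeePower and destroys itself.
; Each tick a sine of game time nudges the Arrow component along Z so it bobs as a marker, with a frame-rate dependent step.
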(event EventInteractionFunction
  ;[1 1 1] Give Player Coffee boost
  (bind _returnvalue (Actor|GetActorOfClass "/Game/BluePrints/GamePlayer.GamePlayer_C"))
  (if (Rendering|IsVisible (Variables|/Game/BluePrints/GamePlayer.GamePlayer_C|Getcoffee _returnvalue))
    (Rendering|SetVisibility (Variables|/Game/BluePrints/GamePlayer.GamePlayer_C|Getcoffee _returnvalue) false false) ; Fade to black animation later
    (Variables|/Game/BluePrints/GamePlayer.GamePlayer_C|SetCoffeePower _returnvalue true)
    (Actor|DestroyActor)))

(event EventTick
  (params (DeltaSeconds :type Float%20%28single-precision%29))
  (Transformation|AddRelativeLocation (Variables|Default|GetArrow) (Math|Vector|MakeVector 0.0 0.0 (* (Math|Trig|Sin(Radians) (Actor|GetGameTimeSinceCreation)) 0.5)) false false))

(fn ConstructionScript)