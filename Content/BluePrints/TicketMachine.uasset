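; Ticket machine actor that serves as the game's exit, usable once the player's Score reaches ScoreMax.
; Overlap shows an interact prompt or a not-enough message based on that score and hides it on leaving.
; Interacting with enough score plays the EndCutscene sequence with movement and look input disabled and removes the HUD.
; Timed delays then show the escape screen and return to the main menu.
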(event Collision|EventActorBeginOverlap
  (params (OtherActor :type Actor%20Object%20Reference))
  ;[1 1 1] Show/Hide Interact Text
  (bind _returnvalue (Actor|GetActorOfClass "/Game/BluePrints/GamePlayer.GamePlayer_C"))
  (if (>= (Variables|/Game/BluePrints/GamePlayer.GamePlayer_C|GetScore _returnvalue) (Variables|/Game/BluePrints/GamePlayer.GamePlayer_C|GetScore_Max _returnvalue))
    (CallFunction|ShowInteractText "Press E to buy ticket")
    (else
      (CallFunction|ShowInteractText "...I don't have enough"))))

(event Collision|EventActorEndOverlap
  (params (OtherActor :type Actor%20Object%20Reference))
  ;[1 1 1] Show/Hide Interact Text
  (CallFunction|HideInteractText))

(event EventInteractionFunction
  (bind _returnvalue (Actor|GetActorOfClass "/Game/BluePrints/GamePlayer.GamePlayer_C"))
  (if (>= (Variables|/Game/BluePrints/GamePlayer.GamePlayer_C|GetScore _returnvalue) (Variables|/Game/BluePrints/GamePlayer.GamePlayer_C|GetScore_Max _returnvalue))
    (CallFunction|HideInteractText)
    (bind _outactor (Sequencer|Player|CreateLevelSequencePlayer "/Game/EndCutscene.EndCutscene" (Utilities|Struct|MakeMovieSceneSequencePlaybackSettings false "(Value=0)" 1.0 0.0 false false true true false false false true)))
    (Sequencer|Player|Play (Variables|/Script/LevelSequence.LevelSequenceActor|GetSequencePlayer _outactor) :!class /Script/MovieScene.MovieSceneSequencePlayer)
    (bind _ashud_default (Utilities|Casting|CastToHudDefault (HUD|GetHUD (Game|GetPlayerController 0))))
    (Widget|RemovefromParent (Variables|/Game/UserInteraface/HudDefault.HudDefault_C|GetPlayerHud _ashud_default))
    (Utilities|FlowControl|Delay 8.0)
    (bind _returnvalue_2 (UserInterface|CreateWidget "/Game/UserInteraface/YouHaveEscapted.YouHaveEscapted_C"))
    (UserInterface|Viewport|AddtoViewport _returnvalue_2 0)
    (Utilities|FlowControl|Delay 6.0)
    (Game|OpenLevel(byObjectReference) "/Game/MainMenu.MainMenu")))

(fn ConstructionScript)